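; BP_Weapon is a base weapon Blueprint that supplies a pickup icon and a crosshair icon to the UI.
; On BeginPlay it sets its pickup widget's image to the weapon's icon and caches BP_HUD from player 0's StellaController.
; An UpdateCrosshair event writes the weapon's crosshair icon to the cached HUD when that reference is valid.
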(event `self.ReceiveBeginPlay`
  (bind _aswbp_pickup (cast `/Game/Blueprints/Widgets/WBP_Pickup` (`WidgetComponent.GetWidget` (`self.PickupWidget`))))
  (`Image.SetBrush` (`/Game/Blueprints/Widgets/WBP_Pickup.Main_Img` _aswbp_pickup) (make `SlateBrush` "Image" "NoTile" "NoMirror" (struct :`X` 32.0 :`Y` 32.0) (struct) (struct :`SpecifiedColor` (struct :`R` 1.0 :`G` 1.0 :`B` 1.0 :`A` 1.0) :`ColorUseRule` "UseColor_Specified") (struct :`CornerRadii` (struct) :`Color` (struct :`SpecifiedColor` (struct) :`ColorUseRule` "UseColor_Specified") :`RoundingType` "HalfHeightRadius") (`self.PickupIcon`)))
  (bind _asstella_controller (cast `StellaController` (`GameplayStatics.GetPlayerController` 0)))
  (bind _asbp_hud (cast `/Game/HUD/BP_HUD` (`PlayerController.GetHUD` _asstella_controller)))
  (set `self.BP HUD` _asbp_hud))

(event `self.UpdateCrosshair`
  (bind _bp_hud (`self.BP HUD`)
    (:`then`
      (set `/Game/HUD/BP_HUD.Crosshair` (`self.CrosshairIcon`) _bp_hud))
    (:`else`)))

(fn `UserConstructionScript`)