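; BP_GruxMolten is a child enemy Blueprint, a molten Grux variant whose destruction ends play.
; On Destroyed, it pauses the game, adds a WBP_End widget to the viewport and shows the player's mouse cursor.
; It adds no other graph logic: BeginPlay, overlap and Tick are disabled stubs, and the construction script only calls the parent.
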(event `self.ReceiveDestroyed`
  (`GameplayStatics.SetGamePaused` true)
  (bind _returnvalue (`|CreateWidget` "/Game/Blueprints/Widgets/Menu/WBP_End.WBP_End_C"))
  (`UserWidget.AddToViewport` _returnvalue 0)
  (set `PlayerController.bShowMouseCursor` true (`GameplayStatics.GetPlayerController` 0)))

(fn `UserConstructionScript`
  (`parent.UserConstructionScript`))